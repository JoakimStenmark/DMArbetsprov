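; PickUp_Base is a pickup actor Blueprint with an optionally spinning static mesh.
; BeginPlay enables or disables Tick based on AnimateModel, and Tick yaws the mesh at RotationSpeed scaled by delta time.
; On EndPlay it passes itself to CallOnPickUpDestroyed on BP_DMArbetsprovGameMode, whatever the reason play ends.
; It contains no overlap or collection logic.
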(event EventBeginPlay
  (Actor|Tick|SetActorTickEnabled (Variables|Default|GetAnimateModel)))

(event Collision|EventActorBeginOverlap
  (params (OtherActor :type Actor%20Object%20Reference)))

(event EventTick
  (params (DeltaSeconds :type Float%20%28single-precision%29))
  (Transformation|AddRelativeRotation (Variables|Default|GetStaticMesh) (Math|Rotator|MakeRotator 0.0 0.0 (* DeltaSeconds (Variables|Default|GetRotationSpeed))) false false))

(event EventEndPlay
  (params (EndPlayReason :type EEndPlayReason%20Enum :default "Destroyed"))
  (bind _asbp_dmarbetsprov_game_mode (Utilities|Casting|CastToBP_DMArbetsprovGameMode (Game|GetGameMode)))
  (Default|CallOnPickUpDestroyed _asbp_dmarbetsprov_game_mode self))

(fn ConstructionScript)