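; PickUp_AmmoPack is an ammo pickup actor that the first-person player collects by walking into it.
; On actor overlap it casts the other actor to BP_FirstPersonCharacter, calls AddAmmo with its AmmoAmount variable, then destroys itself.
; Any other overlapping actor fails the cast and leaves the pack in place.
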(event EventBeginPlay
  (|CallParentFunction) ; This node is disabled and will not be called.\nDrag off pins to build functionality.
)

(event Collision|EventActorBeginOverlap
  (params (OtherActor :type Actor%20Object%20Reference))
  (|CallParentFunction OtherActor)
  (bind _asbp_first_person_character (Utilities|Casting|CastToBP_FirstPersonCharacter OtherActor))
  (Class|DMArbetsprovCharacter|AddAmmo _asbp_first_person_character (Variables|Default|GetAmmoAmount))
  (Actor|DestroyActor))

(event EventTick
  (params (DeltaSeconds :type Float%20%28single-precision%29))
  (|CallParentFunction DeltaSeconds) ; This node is disabled and will not be called.\nDrag off pins to build functionality.
)

(fn ConstructionScript
  (|CallParentFunction))