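; BP_Enemy is an AI-moved enemy that heads for a target location and can be knocked back and destroyed.
; It starts moving after a post-spawn delay and reissues the move when it leaves a BP_GoalZone.
; Point and radial damage reduce health and apply damage-type-scaled impulses, radial ones away from the origin.
; At zero health it notifies BP_DMArbetsprovGameMode and destroys itself, with debug prints along the way.
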(event OnComponentEndOverlap(CapsuleComponent)
  (params (OverlappedComponent :type Primitive%20Component%20Object%20Reference) (OtherActor :type Actor%20Object%20Reference) (OtherComp :type Primitive%20Component%20Object%20Reference) (OtherBodyIndex :type Integer))
  (Utilities|Casting|CastToBP_GoalZone OtherActor)
  (AI|AIMoveTo self (Variables|Default|GetTargetLocation) 0 1e+02 false))

(event EventBeginPlay
  (Utilities|FlowControl|Delay (Variables|Default|GetPostSpawnDelay))
  (AI|AIMoveTo self (Variables|Default|GetTargetLocation) 0 1e+02 false))

(event Game|Damage|EventRadialDamage
  (params (DamageReceived :type Float%20%28single-precision%29) (DamageType :type Damage%20Type%20Object%20Reference) (Origin :type Vector :default "0, 0, 0") (HitInfo :type Hit%20Result%20Structure%20%28by%20ref%29) (InstigatedBy :type Controller%20Object%20Reference) (DamageCauser :type Actor%20Object%20Reference))
  (bind _self self)
  (Variables|Default|SetCurrentHealth (- (Variables|Default|GetCurrentHealth) DamageReceived))
  (Physics|AddImpulse (Variables|Character|GetCharacterMovement) (* (Math|Vector|Normalize (* (- Origin (Transformation|GetWorldLocation (Variables|Default|GetCapsuleComponent))) -1.0)) (Variables|/Script/Engine.DamageType|GetDamageImpulse DamageType)) false)
  (Development|PrintString (Utilities|String|BuildString(Float) "Enemy Health: " "" (Variables|Default|GetCurrentHealth)))
  (if (<= (Variables|Default|GetCurrentHealth) 0.0)
    (bind _asbp_dmarbetsprov_game_mode (Utilities|Casting|CastToBP_DMArbetsprovGameMode (Game|GetGameMode)))
    (Default|CallOnEnemyDestroyed _asbp_dmarbetsprov_game_mode _self)
    (Development|PrintString (Utilities|String|Append (Utilities|GetDisplayName _self) "Was Destroyed"))
    (Actor|DestroyActor)))

(event Game|Damage|EventPointDamage
  (params (Damage :type Float%20%28single-precision%29) (DamageType :type Damage%20Type%20Object%20Reference) (HitLocation :type Vector :default "0, 0, 0") (HitNormal :type Vector :default "0, 0, 0") (HitComponent :type Primitive%20Component%20Object%20Reference) (BoneName :type Name :default "None") (ShotFromDirection :type Vector :default "0, 0, 0") (InstigatedBy :type Controller%20Object%20Reference) (DamageCauser :type Actor%20Object%20Reference) (HitInfo :type Hit%20Result%20Structure%20%28by%20ref%29))
  (bind _self self)
  (Variables|Default|SetCurrentHealth (- (Variables|Default|GetCurrentHealth) Damage))
  (Physics|AddImpulse (Variables|Character|GetCharacterMovement) (* (* HitNormal (Variables|/Script/Engine.DamageType|GetDamageImpulse DamageType)) -1.0) false)
  (Development|PrintString (Utilities|String|BuildString(Float) "Enemy Health: " "" (Variables|Default|GetCurrentHealth)))
  (if (<= (Variables|Default|GetCurrentHealth) 0.0)
    (bind _asbp_dmarbetsprov_game_mode (Utilities|Casting|CastToBP_DMArbetsprovGameMode (Game|GetGameMode)))
    (Default|CallOnEnemyDestroyed _asbp_dmarbetsprov_game_mode _self)
    (Development|PrintString (Utilities|String|Append (Utilities|GetDisplayName _self) "Was Destroyed"))
    (Actor|DestroyActor)))

(fn ConstructionScript)