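; Enemy spawner actor that populates an area with AI enemies when play begins.
; On BeginPlay it loops over EnemyAmount and spawns the EnemyToSpawn class at random navigable points around the root's location.
; The Sphere component's radius sets the spawn area.
; Each spawned pawn gets a random yaw, and overlap, tick and construction logic are empty.
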(event EventBeginPlay
  (for _index (range 0 (Variables|Default|GetEnemyAmount))
    (AI|SpawnAIFromClass (Variables|Default|GetEnemyToSpawn) 0 (.RandomLocation (Class|NavigationSystemV1|GetRandomPointinNavigableRadius (Transformation|GetWorldLocation (Variables|Default|GetDefaultSceneRoot)) (Variables|/Script/Engine.SphereComponent|GetSphereRadius (Variables|Default|GetSphere)) 0 0)) (Math|Rotator|MakeRotator 0.0 0.0 (Math|Random|RandomFloatinRange 0.0 359.0)) false)))

(event Collision|EventActorBeginOverlap
  (params (OtherActor :type Actor%20Object%20Reference)))

(event EventTick
  (params (DeltaSeconds :type Float%20%28single-precision%29)))

(fn ConstructionScript)