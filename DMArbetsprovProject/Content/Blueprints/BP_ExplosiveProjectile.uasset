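; Explosive projectile that deals radial damage when it hits something.
; On Hit it applies full damage within ExplosiveRadius around its Sphere component, instigated by player controller 0, and briefly draws a red debug sphere if damage lands.
; The explosion particle spawns separately on EndPlay at the actor's location, and this graph never destroys the actor itself.
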(event EventBeginPlay)

(event Collision|EventActorBeginOverlap
  (params (OtherActor :type Actor%20Object%20Reference)))

(event EventTick
  (params (DeltaSeconds :type Float%20%28single-precision%29)))

(event EventEndPlay
  (params (EndPlayReason :type EEndPlayReason%20Enum :default "Destroyed"))
  (Effects|SpawnEmitteratLocation "/Game/StarterContent/Particles/P_Explosion.P_Explosion" (Transformation|GetActorLocation)))

(event Collision|EventHit
  (params (MyComp :type Primitive%20Component%20Object%20Reference) (Other :type Actor%20Object%20Reference) (OtherComp :type Primitive%20Component%20Object%20Reference) (bSelfMoved :type Boolean) (HitLocation :type Vector :default "0, 0, 0") (HitNormal :type Vector :default "0, 0, 0") (NormalImpulse :type Vector :default "0, 0, 0") (Hit :type Hit%20Result%20Structure%20%28by%20ref%29))
  (bind _sphere (Variables|Default|GetSphere))
  (bind _returnvalue (Transformation|GetWorldLocation _sphere))
  (bind _returnvalue_2 (Game|Damage|ApplyRadialDamage (Variables|Default|GetBaseDamage) _returnvalue (Variables|Default|GetExplosiveRadius) (Variables|Default|GetDamageType) 0 self (Game|GetPlayerController 0) true "ECC_Visibility"))
  (if _returnvalue_2
    (Rendering|Debug|DrawDebugSphere _returnvalue (Variables|Default|GetExplosiveRadius) 12 "(R=1.000000,G=0.000000,B=0.008760,A=1.000000)" 1.0)))

(fn ConstructionScript)