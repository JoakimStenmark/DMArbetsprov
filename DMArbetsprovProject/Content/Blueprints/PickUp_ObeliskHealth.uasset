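; Pickup Blueprint that, judging by its names, repairs the obelisk by adjusting the game's lose condition.
; On actor overlap it runs the parent's overlap logic, then casts the game mode to BP_DMArbetsprovGameMode and passes ObeliskRepairAmount to ChangeLoseCondition.
; This graph does not check which actor overlapped, and its construction script only calls the parent.
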(event EventBeginPlay
  (|CallParentFunction) ; This node is disabled and will not be called.\nDrag off pins to build functionality.
)

(event Collision|EventActorBeginOverlap
  (params (OtherActor :type Actor%20Object%20Reference))
  (|CallParentFunction OtherActor)
  (bind _asbp_dmarbetsprov_game_mode (Utilities|Casting|CastToBP_DMArbetsprovGameMode (Game|GetGameMode)))
  (Default|ChangeLoseCondition _asbp_dmarbetsprov_game_mode (Variables|Default|GetObeliskRepairAmount)))

(event EventTick
  (params (DeltaSeconds :type Float%20%28single-precision%29))
  (|CallParentFunction DeltaSeconds) ; This node is disabled and will not be called.\nDrag off pins to build functionality.
)

(fn ConstructionScript
  (|CallParentFunction))