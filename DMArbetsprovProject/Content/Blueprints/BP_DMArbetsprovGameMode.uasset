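; Game mode that runs the match flow: start menu, objective HUD, spawners and game over.
; PostLogin opens a UI-only start menu and adds the HUD; StartGame closes the menu, restores game input and spawns enemy and pickup spawners.
; Destroyed events, bound on start and unbound on EndPlay, remove dead actors from each spawner's list.
; ChangeLoseCondition updates the objective bar and shows game over once when it reaches zero.
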(event Custom|OnEnemyDestroyed_Event
  (params (DeadEnemy :type BP%20Enemy%20Object%20Reference))
  ;[1 1 1] Start Listening for Events
  (Class|ActorSpawner|RemoveActorfromSpawnedActorsList (Variables|Default|GetEnemySpawner) DeadEnemy))

(event Custom|StartGame
  (CallFunction|CloseStartMenu)
  (Utilities|FlowControl|Sequence
    (:then_0
      ;[1 1 1] Start Listening for Events
      (EventDispatchers|BindEventtoOnEnemyDestroyed (delegate Custom|OnEnemyDestroyed_Event))
      (EventDispatchers|BindEventtoOnPickUpDestroyed (delegate Custom|OnPickUpDestroyed_Event)))
    (:then_1
      ;[1 1 1] Spawn Spawners
      (bind _returnvalue (Game|SpawnActorfromClass "/Game/Blueprints/BP_Spawner_Enemy.BP_Spawner_Enemy_C" (Variables|Default|GetDefaultPosition) "AlwaysSpawn" 0 0))
      (Variables|Default|SetEnemySpawner _returnvalue)
      (bind _returnvalue_2 (Game|SpawnActorfromClass "/Game/Blueprints/BP_Spawner_PickUp.BP_Spawner_PickUp_C" (Variables|Default|GetDefaultPosition) "AlwaysSpawn" 0 0))
      (Variables|Default|SetPickupSpawner _returnvalue_2))))

(event Custom|OnPickUpDestroyed_Event
  (params (DestroyedPickUp :type Pick%20Up%20Base%20Object%20Reference))
  ;[1 1 1] Start Listening for Events
  (Class|ActorSpawner|RemoveActorfromSpawnedActorsList (Variables|Default|GetPickupSpawner) DestroyedPickUp))

(event Custom|ChangeLoseCondition
  (params (Amount :type Float%20%28single-precision%29))
  (bind _output_get (Variables|Default|SetCurrentLoseCondition (+ (Variables|Default|GetCurrentLoseCondition) Amount)))
  (Default|UpdateObjectiveBar (Variables|Default|GetObjectiveHUD) (Math|Float|NormalizetoRange _output_get 0.0 (Variables|Default|GetInitialLoseCondition)))
  (if (<= (Variables|Default|GetCurrentLoseCondition) 0.0)
    (Utilities|FlowControl|DoOnce false
      (:Completed
        (Default|ShowGameOver (Variables|Default|GetObjectiveHUD))))))

(event EventEndPlay
  (params (EndPlayReason :type EEndPlayReason%20Enum :default "Destroyed"))
  (EventDispatchers|UnbindallEventsfromOnEnemyDestroyed)
  (EventDispatchers|UnbindallEventsfromOnPickUpDestroyed))

(event EventPostLogin
  (params (NewPlayer :type Player%20Controller%20Object%20Reference))
  (CallFunction|OpenStartMenu)
  (bind _returnvalue (UserInterface|CreateWidget "/Game/Blueprints/UMG_ObjectiveHUD.UMG_ObjectiveHUD_C"))
  (bind _output_get (Variables|Default|SetObjectiveHUD _returnvalue))
  (UserInterface|Viewport|AddtoViewport _output_get 1))

(fn ConstructionScript)

(fn OpenStartMenu
  (bind _returnvalue (Game|GetPlayerController 0))
  (bind _returnvalue_2 (UserInterface|CreateWidget "/Game/Blueprints/UMG_StartMenu.UMG_StartMenu_C"))
  (bind _output_get (Variables|Default|SetStartMenu _returnvalue_2))
  (Input|SetInputModeUIOnly _returnvalue 0 "DoNotLock")
  (UserInterface|Viewport|AddtoViewport _output_get 0)
  (Variables|/Script/Engine.PlayerController|SetbShowMouseCursor _returnvalue true))

(fn CloseStartMenu
  (bind _returnvalue (Game|GetPlayerController 0))
  (Utilities|IsValid (Variables|Default|GetStartMenu)
    (:Is%20Valid
      (Widget|RemovefromParent (Variables|Default|GetStartMenu))
      (Variables|Default|SetStartMenu 0))
    (:Is%20Not%20Valid
      _))
  (Input|SetInputModeGameOnly _returnvalue)
  (Variables|/Script/Engine.PlayerController|SetbShowMouseCursor _returnvalue false))