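; Enemy spawner that places enemies on random navmesh points and sends them toward goal zones.
; On BeginPlay it caches all BP_GoalZone actors, spawns an initial batch, then starts a looping timer that reuses the same spawn path.
; Each spawned BP_Enemy receives a random zone's location as TargetLocation.
; The random index is rolled separately for validation and assignment, and its Length-1 bound excludes the last zone.
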(event Custom|Event%20Spawn%20Actor
  (bind _goalzones (Variables|Default|GetGoalZones))
  (bind _returnvalue (Utilities|Array|Length _goalzones))
  (bind _returnvalue_2 (- _returnvalue 1))
  (bind _returnvalue_3 (Math|Random|RandomInteger _returnvalue_2))
  (bind _output (Utilities|Array|Get(acopy) _goalzones _returnvalue_3))
  ;[1 1 1] Start Spawning over time
  (bind _returnvalue_4 (Class|ActorSpawner|SpawnActoronRandomNavMeshPoint))
  ;[1 1 1] Give spawned enemy a target to go to
  (bind _asbp_enemy (Utilities|Casting|CastToBP_Enemy _returnvalue_4))
  (if (Utilities|IsValid _output)
    (Variables|/Game/Blueprints/BP_Enemy.BP_Enemy_C|SetTargetLocation _asbp_enemy (Transformation|GetActorLocation _output))))

(event EventBeginPlay
  (Utilities|FlowControl|Sequence
    (:then_0
      ;[1 1 1] Find target that enemies can go to
      (bind _outactors (Actor|GetAllActorsOfClass "/Game/Blueprints/BP_GoalZone.BP_GoalZone_C"))
      (Variables|Default|SetGoalZones _outactors))
    (:then_1
      (for _index (range 0 3)
        (bind _returnvalue (Class|ActorSpawner|SpawnActoronRandomNavMeshPoint))
        ;[1 1 1] Give spawned enemy a target to go to
        (bind _asbp_enemy (Utilities|Casting|CastToBP_Enemy _returnvalue))
        (if (Utilities|IsValid (Utilities|Array|Get(acopy) (Variables|Default|GetGoalZones) (Math|Random|RandomInteger (- (Utilities|Array|Length (Variables|Default|GetGoalZones)) 1))))
          (Variables|/Game/Blueprints/BP_Enemy.BP_Enemy_C|SetTargetLocation _asbp_enemy (Transformation|GetActorLocation (Utilities|Array|Get(acopy) (Variables|Default|GetGoalZones) (Math|Random|RandomInteger (- (Utilities|Array|Length (Variables|Default|GetGoalZones)) 1))))))))
    (:then_2
      ;[1 1 1] Start Spawning over time
      (Utilities|Time|SetTimerbyEvent (delegate Custom|Event%20Spawn%20Actor) (Variables|Default|GetTimeBetweenSpawns) true))))

(fn ConstructionScript)