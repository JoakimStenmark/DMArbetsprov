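; BP_GoalZone is a goal area that drains the game mode's lose condition while enemies occupy it.
; Cube overlap events count BP_Enemy actors entering and leaving, switching the cube and static mesh to an occupied material and back once the zone empties.
; While the count is above zero, Tick calls ChangeLoseCondition on the cached BP_DMArbetsprovGameMode with negative delta time, so the drain is time-based regardless of enemy count.
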(event OnComponentBeginOverlap(Cube)
  (params (OverlappedComponent :type Primitive%20Component%20Object%20Reference) (OtherActor :type Actor%20Object%20Reference) (OtherComp :type Primitive%20Component%20Object%20Reference) (OtherBodyIndex :type Integer) (bFromSweep :type Boolean) (SweepResult :type Hit%20Result%20Structure%20%28by%20ref%29))
  ;[1 1 1] Detect Enemies entering and Leaving
  (Utilities|Casting|CastToBP_Enemy OtherActor)
  (Math|Integer|IncrementInt (Variables|Default|GetEnemiesInside)
    (:%20%20
      (Rendering|Material|SetMaterial (Variables|Default|GetCube) 0 "/Game/Materials/MatInst_GoalOccupied.MatInst_GoalOccupied")
      (Rendering|Material|SetMaterial (Variables|Default|GetStaticMesh) 0 "/Game/Materials/MatInst_GoalOccupied.MatInst_GoalOccupied"))))

(event OnComponentEndOverlap(Cube)
  (params (OverlappedComponent :type Primitive%20Component%20Object%20Reference) (OtherActor :type Actor%20Object%20Reference) (OtherComp :type Primitive%20Component%20Object%20Reference) (OtherBodyIndex :type Integer))
  ;[1 1 1] Detect Enemies entering and Leaving
  (Utilities|Casting|CastToBP_Enemy OtherActor)
  (bind _result (Math|Integer|DecrementInt (Variables|Default|GetEnemiesInside))
    (:%20%20
      (if (< _result 1)
        (Rendering|Material|SetMaterial (Variables|Default|GetCube) 0 "/Game/Materials/MatInst_Goal.MatInst_Goal")
        (Rendering|Material|SetMaterial (Variables|Default|GetStaticMesh) 0 "/Game/Materials/MatInst_Goal.MatInst_Goal")))))

(event EventTick
  (params (DeltaSeconds :type Float%20%28single-precision%29))
  ;[1 1 1] Update Lose condition if enemies inside
  (if (> (Variables|Default|GetEnemiesInside) 0)
    (Default|ChangeLoseCondition (Variables|Default|GetGameMode) (* DeltaSeconds -1.0))))

(event EventBeginPlay
  (bind _asbp_dmarbetsprov_game_mode (Utilities|Casting|CastToBP_DMArbetsprovGameMode (Game|GetGameMode)))
  (bind _output_get (Variables|Default|SetGameMode _asbp_dmarbetsprov_game_mode))
  (Development|PrintString (Utilities|GetDisplayName _output_get)))

(fn ConstructionScript)