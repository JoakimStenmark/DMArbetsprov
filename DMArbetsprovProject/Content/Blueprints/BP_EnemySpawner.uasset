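; Enemy spawner that populates the level at BeginPlay by calling SpawnActorOnRandomNavMeshPoint in a loop sized by ActorAmountLimit.
; The spawn function and enemy-destroyed binding are used here but defined outside these graphs.
; The destroyed callback removes the dead actor from SpawnedActors and prints a removal message on success, without spawning a replacement.
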(event Custom|OnEnemyDestroyed_Event
  (params (DeadActor :type Actor%20Object%20Reference))
  (bind _returnvalue (Utilities|Array|RemoveItem (Variables|Default|GetSpawnedActors) DeadActor))
  (if _returnvalue
    (Development|PrintString (Utilities|String|Append (Utilities|GetDisplayName 0) " Was Removed"))))

(event EventBeginPlay
  (EventDispatchers|BindEventtoOnEnemyDestroyed (delegate Custom|OnEnemyDestroyed_Event))
  (for _index (range 0 (Variables|Default|GetActorAmountLimit))
    (Class|ActorSpawner|SpawnActoronRandomNavMeshPoint)))

(fn ConstructionScript)